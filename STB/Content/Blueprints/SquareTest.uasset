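; SquareTest is a test Blueprint that drives procedural mesh generation through its BaseMesh.
; StartEvent passes scale, triangle, vertex, vertex collider, normal, UV, tangent and vertex colour data into BaseMesh, then creates the mesh.
; UpdateEvent forwards the shape's side count and collider mesh to BaseMesh to update it.
; The construction script is empty, and all mesh-building logic is delegated to BaseMesh.
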(event EventStartEvent
  (bind _basemesh (Variables|Default|GetBaseMesh))
  (Class|ProGenMeshBase|UpdateAllComponents _basemesh (Variables|Default|GetObjectScale) (Variables|Default|GetTriangles) (Variables|Default|GetVerticies) (Variables|Default|GetVertexColliders) (Variables|Default|GetNormals) (Variables|Default|GetUV0) (Variables|Default|GetTangents) (Variables|Default|GetVertexColours))
  (Class|ProGenMeshBase|CreateMesh _basemesh))

(event EventUpdateEvent
  (params (SidesOnShape :type Integer) (ColliderMesh :type Static%20Mesh%20Object%20Reference))
  (Class|ProGenMeshBase|UpdateMesh (Variables|Default|GetBaseMesh) SidesOnShape ColliderMesh))

(fn ConstructionScript)